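; Player spaceship Blueprint that turns mobile device motion into horizontal and vertical velocity values.
; On BeginPlay it calls an Android API template function to check whether the phone has an accelerometer.
; Each Tick derives both velocities and a CurrentGravity value from motion gravity when one is present, otherwise from tilt, with separate offsets and scales.
; The graph only sets these variables and does not move the ship itself.
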(event `self.ReceiveBeginPlay`
  (set `self.hasAccel` (`AndroidAPITemplateFunctions.AndroidAPITemplate_DoesPhoneHaveAccel`)))

(event `self.ReceiveTick`
  (params (DeltaSeconds :type "Float (single-precision)"))
  (bind (_tilt _rotationrate _gravity) (`PlayerController.GetInputMotionState` (`GameplayStatics.GetPlayerController` 0)))
  (bind _returnvalue (+ (.x _tilt) 0.75))
  (bind _returnvalue_2 (+ (.y _gravity) -6.0))
  (if (`self.hasAccel`)
    (set `self.horizontalVelocity` (* (.x _gravity) -150.0))
    (set `self.verticalVelocity` (* _returnvalue_2 -200.0))
    (set `self.currentGravity` (+ (* -1 _returnvalue_2) -2.0))
    (else
      (set `self.verticalVelocity` (* _returnvalue 900.0))
      (set `self.horizontalVelocity` (* (.y _tilt) 1500.0))
      (set `self.currentGravity` _returnvalue))))

(fn `UserConstructionScript`)